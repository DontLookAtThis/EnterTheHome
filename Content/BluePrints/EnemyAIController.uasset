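; AI controller for EnemyBP that wanders between random points in a fixed rectangle and reacts to player proximity.
; Each tick it moves toward the current point while alive and unstunned, otherwise stops, and rerolls on arrival, failure or near-zero velocity.
; When moving near the game mode's PlayerRef, it retargets using a jittered away-from-player vector, scaled but not added to the pawn's location.
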(event `self.ReceiveBeginPlay`
  (`self.SetNewRandomLocation`))

(event `self.ReceiveTick`
  (params (DeltaSeconds :type "Float (single-precision)"))
  (bind _returnvalue (`KismetMathLibrary.RandomFloatInRange` -0.1 0.1))
  (bind _returnvalue_2 (`self.K2_GetPawn`))
  (bind _asenemy_bp (cast `/Game/BluePrints/EnemyBP` (`self.K2_GetPawn`)))
  (if (and (`Enemy.IsAlive` _asenemy_bp) (not (`/Game/BluePrints/EnemyBP.Stunned` _asenemy_bp)))
    (bind _returnvalue_3 (`self.MoveToLocation` (`self.CurrentMoveToLocation`) -1.0 true true false true null))
    (if (or (`|EnumEquality` _returnvalue_3 "AlreadyAtGoal") (`|EnumEquality` _returnvalue_3 "Failed"))
      (`self.SetNewRandomLocation` :!label _label)
      (elif (< (`KismetMathLibrary.VSize` (`self.GetVelocity` _returnvalue_2)) 10.0)
        (goto _label)
        (else
          (bind _asenter_the_home_game_mode_base_bp (cast `/Game/BluePrints/EnterTheHomeGameModeBase_BP` (`GameplayStatics.GetGameMode`)))
          (bind _playerref (`/Game/BluePrints/EnterTheHomeGameModeBase_BP.PlayerRef` _asenter_the_home_game_mode_base_bp))
          (`/Engine/EditorBlueprintResources/StandardMacros.IsValid` _playerref
            (:`Is Valid`
              (bind _returnvalue_4 (- (`self.K2_GetActorLocation` _returnvalue_2) (`self.K2_GetActorLocation` _playerref)))
              (if (< (`KismetMathLibrary.VSize` _returnvalue_4) (`self.CloseToPlayer`))
                (set `self.CurrentMoveToLocation` (* (+ (`KismetMathLibrary.Normal` _returnvalue_4) (`KismetMathLibrary.MakeVector` _returnvalue _returnvalue)) 100.0))
                (`KismetSystemLibrary.PrintString` "In Range of player" true true (struct :`G` 0.66 :`B` 1.0 :`A` 1.0) 0.001)))))))
    (else
      (`self.StopMovement`))))

(fn `SetNewRandomLocation`
  (set `self.CurrentMoveToLocation` (`KismetMathLibrary.MakeVector` (`KismetMathLibrary.RandomFloatInRange` -800.0 1200.0) (`KismetMathLibrary.RandomFloatInRange` -1300.0 1300.0))))

(fn `UserConstructionScript`)