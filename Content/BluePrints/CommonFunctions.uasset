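; CommonFunctions is a set of shared UMG helper functions for images and button focus highlighting.
; SetImage swaps an image's brush texture and sizes it to the texture's dimensions, keeping its margin, draw mode, tiling and mirroring.
; SetButtonsHovered loops over button and brush pairs, using the hovered brush as the normal style for any button with the given player controller's user focus and restoring the normal brush on the rest.
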(fn `SetButtonsHovered`
  (params (`Button In` :type "Array of /Game/BluePrints/ButtonImage Structure") (PC :type "PlayerController Object Reference"))
  (for _array_element `Button In`
    (if (`Widget.HasUserFocus` (break `/Game/BluePrints/ButtonImage` _array_element) PC)
      (bind (_normal _hovered _pressed) (break `ButtonStyle` (`.ButtonBrush_5_BD9658A24CCFAC68757ED2BB395E6DA8` (break `/Game/BluePrints/ButtonImage` _array_element))))
      (`Button.SetStyle` (break `/Game/BluePrints/ButtonImage` _array_element) (make `ButtonStyle` _hovered _hovered _pressed))
      (else
        (`Button.SetStyle` (break `/Game/BluePrints/ButtonImage` _array_element) (make `ButtonStyle` _normal _hovered _pressed))))))

(fn `SetImage`
  (params (ImageObject :type "Image Object Reference") (TextureImage :type "Texture2D Object Reference"))
  (bind (_brush_imagesize _brush_margin _brush_tintcolor _brush_resourceobject _brush_drawas _brush_tiling _brush_mirroring) (break `SlateBrush` (`Image.Brush` ImageObject)))
  (`Image.SetBrush` ImageObject (make `SlateBrush` (`KismetMathLibrary.MakeVector2D` (`KismetMathLibrary.Conv_IntToDouble` (`Texture2D.Blueprint_GetSizeX` TextureImage)) (`KismetMathLibrary.Conv_IntToDouble` (`Texture2D.Blueprint_GetSizeY` TextureImage))) _brush_margin (struct :`SpecifiedColor` (struct :`R` 1.0 :`G` 1.0 :`B` 1.0 :`A` 1.0) :`ColorUseRule` "UseColor_Specified") TextureImage _brush_drawas _brush_tiling _brush_mirroring)))