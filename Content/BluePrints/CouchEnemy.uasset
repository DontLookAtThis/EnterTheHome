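; CouchEnemy is the couch variant of an enemy Blueprint, leaving most behavior to its parent class.
; On BeginPlay it runs the parent logic, attaches OutsidePossessedMesh to the main cushion socket on Mesh with world transform kept, and zeroes the world rotation of OGLocationOutline.
; Overlap and construction only call the parent, and Tick is disabled.
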(event `self.ReceiveBeginPlay`
  (`parent.ReceiveBeginPlay`)
  (`SceneComponent.K2_AttachToComponent` (`self.OutsidePossessedMesh`) (`self.Mesh`) "Couch_CushionMain" "KeepWorld" "KeepWorld" "KeepWorld" true)
  (`SceneComponent.K2_SetWorldRotation` :`self` (`self.OGLocationOutline`)))

(event `self.ReceiveActorBeginOverlap`
  (params (OtherActor :type "Actor Object Reference"))
  (`parent.ReceiveActorBeginOverlap` OtherActor))

(fn `UserConstructionScript`
  (`parent.UserConstructionScript`))